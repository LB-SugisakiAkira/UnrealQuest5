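; Timed bomb actor that detonates a few seconds after it spawns.
; On BeginPlay its Sphere uses physics-only collision during the fuse, then expands into a blast radius and switches to query-only collision.
; It spawns the NS_Bomb Niagara effect at the mesh location and destroys itself shortly afterward.
; The graph has no damage or overlap handling of its own.
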(event EventBeginPlay
  (bind _sphere (Variables|Default|GetSphere))
  (Collision|SetCollisionEnabled (Variables|Default|GetSphere) "PhysicsOnly")
  (Utilities|FlowControl|Delay 3.0)
  (Components|Sphere|SetSphereRadius _sphere 256.0 true)
  (Collision|SetCollisionEnabled _sphere "QueryOnly")
  (Niagara|SpawnSystematLocation "/Game/UnrealQuest5/Effects/NS_Bomb.NS_Bomb" (Transformation|GetWorldLocation (Variables|Default|GetStaticMesh)))
  (Utilities|FlowControl|Delay 0.5)
  (Actor|DestroyActor))

(fn ConstructionScript)