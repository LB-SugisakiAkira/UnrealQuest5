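; Enemy character for UnrealQuest5 that swings a blade and is defeated by a single hit from the player's blade.
; Attack plays a montage, using delays to enable blade collision only during the swing, excluding wind-up and recovery.
; A capsule overlap with a PlayerBladeAttack-tagged component sets IsDefeated, which blocks further attacks and hits, and plays a damage montage.
; When that montage completes, the mesh ragdolls and BP_UQ5_GameMode is notified via AttackEnemy.
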(event OnComponentBeginOverlap(CapsuleComponent)
  (params (OverlappedComponent :type Primitive%20Component%20Object%20Reference) (OtherActor :type Actor%20Object%20Reference) (OtherComp :type Primitive%20Component%20Object%20Reference) (OtherBodyIndex :type Integer) (bFromSweep :type Boolean) (SweepResult :type Hit%20Result%20Structure%20%28by%20ref%29))
  (bind _mesh (Variables|Character|GetMesh))
  (if (Components|ComponentHasTag OtherComp "PlayerBladeAttack")
    (if (not (Variables|Default|GetIsDefeated))
      (Development|PrintString "PlayerAttacked")
      (Variables|Default|SetIsDefeated true)
      (Animation|Montage|PlayMontage (Variables|Character|GetMesh) "/Game/UnrealQuest5/Characters/Mannequins/Animations/UQ5/AM_Damaged.AM_Damaged"
        (:OnCompleted
          (Class|SkeletalMeshComponent|SetAllBodiesSimulatePhysics _mesh true)
          (Collision|SetCollisionEnabled _mesh "PhysicsOnly")
          (bind _asbp_uq5_game_mode (Utilities|Casting|CastToBP_UQ5_GameMode (Game|GetGameMode)))
          (Default|AttackEnemy _asbp_uq5_game_mode))))))

(event Custom|Attack
  ;[1 0 0 0.5] 攻撃
  (if (not (Variables|Default|GetIsDefeated))
    (Animation|Montage|PlayMontage (Variables|Character|GetMesh) "/Game/UnrealQuest5/Characters/Mannequins/Animations/UQ5/AM_Enemy_Attack01.AM_Enemy_Attack01"
      (:then
        (Utilities|FlowControl|Delay 0.2) ; 振り被った動きでは当たり判定を有効にしないため
        (Collision|SetCollisionEnabled (Variables|Default|GetBladeCollision) "QueryOnly")
        (Utilities|FlowControl|Delay 0.4) ; 振り終わって構え直す間もオフにしたいのでOnCompletedではなくDelayで繋げる
        (Collision|SetCollisionEnabled (Variables|Default|GetBladeCollision) "NoCollision")))))

(fn ConstructionScript)